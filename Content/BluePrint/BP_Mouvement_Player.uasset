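; Player character Blueprint that handles horizontal movement and animation for a flipbook-based sprite.
; The MoveRight axis adds movement input along world X.
; Each tick, UpdateAnimation switches the sprite between run and idle flipbooks based on whether velocity is non-zero.
; UpdateControlAnimation compares X velocity to zero but drives nothing and is not called in this graph.
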(event Custom|UpdateAnimation
  (Sprite|SetFlipbook (Variables|Default|GetSprite) (select (> (Math|Vector|VectorLength (Variables|/Script/Engine.MovementComponent|GetVelocity (Variables|Character|GetCharacterMovement))) 0.0) "/Game/Asset/sprites/player/run/player-run.player-run" "/Game/Asset/sprites/player/idle/player-idle.player-idle")))

(event Custom|UpdateControlAnimation
  (Math|Float|CompareFloat (.X (Math|Vector|BreakVector (Variables|/Script/Engine.MovementComponent|GetVelocity (Variables|Character|GetCharacterMovement)))) 0.0))

(event EventTick
  (params (DeltaSeconds :type Float%20%28single-precision%29))
  (CallFunction|UpdateAnimation))

(event Input|AxisEvents|InputAxisMoveRight
  (params (AxisValue :type Float%20%28single-precision%29))
  (Pawn|Input|AddMovementInput "1.000000,0.000000,0.000000" AxisValue false))

(fn ConstructionScript)